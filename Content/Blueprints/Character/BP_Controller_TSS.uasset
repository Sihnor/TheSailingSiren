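; Player controller that owns the inventory UI and a first-screen overlay.
; BeginPlay adds both widgets to the viewport with the inventory collapsed; DisableFirstScreen later collapses the AlmostBlack overlay.
; ShowInventory runs the parent logic, then, based on IsInInventory, either shows the widget and fills it with item icons from BP_CharacterState's inventory, or collapses and clears it.
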(event `self.ReceiveBeginPlay`
  (bind _returnvalue (`|CreateWidget` "/Game/Blueprints/UI/WBP_Inventory.WBP_Inventory_C" self))
  (bind _output_get (set `self.InventoryWidget` _returnvalue))
  (`UserWidget.AddToViewport` _output_get 0)
  (set `Widget.Visibility` "Collapsed" (`self.InventoryWidget`))
  (bind _returnvalue_2 (`|CreateWidget` "/Game/Blueprints/UI/WBP_AlmostBlack.WBP_AlmostBlack_C" self))
  (bind _output_get_2 (set `self.AlmostBlackWidget` _returnvalue_2))
  (`UserWidget.AddToViewport` _output_get_2 0))

(event `self.ShowInventory`
  (`parent.ShowInventory`)
  (if (`self.bIsInInventory`)
    (set `Widget.Visibility` "Visible" (`self.InventoryWidget`))
    (bind _asbp_character_state (cast `/Game/Blueprints/Character/BP_CharacterState` (`GameplayStatics.GetPlayerState` 0)))
    (for _array_element (`CharacterState.Inventory` _asbp_character_state)
      (bind _returnvalue (`Item.GetItemIcon` (cast `Item` _array_element :!pure true)))
      (`/Game/Blueprints/UI/WBP_Inventory.SetInventoryItem` (`self.InventoryWidget`) _returnvalue))
    (else
      (set `Widget.Visibility` "Collapsed" (`self.InventoryWidget`))
      (`/Game/Blueprints/UI/WBP_Inventory.ClearInventory` (`self.InventoryWidget`)))))

(fn `DisableFirstScreen`
  (set `Widget.Visibility` "Collapsed" (`self.AlmostBlackWidget`)))

(fn `UserConstructionScript`)