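; Game mode for TSS that scripts the narrative of a riddle game, from introduction through Mot and Samael dialogues, letter reading and closing monologues.
; Story events, several extending parent handlers, spawn voice audio components chained through OnAudioFinished to play lines sequentially and trigger later beats.
; It drives the cached player controller to toggle input, letter widget and monologue state.
; Solved riddles play a random sound, with RiddleFour also granting a Match.
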(event `self.ReceiveBeginPlay`
  (bind _asbp_controller_tss (cast `/Game/Blueprints/Character/BP_Controller_TSS` (`GameplayStatics.GetPlayerController` 0)))
  (set `self.PlayerController` _asbp_controller_tss))

(event `self.OnRiddleSolved`
  (params (CurrentRiddleIndex :type "ECurrentPlayState Enum" :default "None"))
  (`parent.OnRiddleSolved` CurrentRiddleIndex))

(event `self.OnStartIntroduction`
  ;[1 1 1] Einleitung
  (`parent.OnStartIntroduction`)
  (`KismetSystemLibrary.Delay` 0.5)
  (`self.OnEndIntroduction` :!label _label)
  (`/Game/Blueprints/Character/BP_Controller_TSS.DisableEyesClosedScreen` (`self.PlayerController`)))

(event `OnAudioFinished_Event`
  ;[1 1 1] Einleitung
  (goto _label))

(event `self.OnEndIntroduction`
  ;[1 1 1] Monolog Samael
  (`parent.OnEndIntroduction`)
  (bind _returnvalue (`AddComponent|NODE_AddAudioComponent-4`))
  (`/Engine/EditorBlueprintResources/StandardMacros.IsValid` _returnvalue
    (:`Is Valid`
      (add `AudioComponent.OnAudioFinished` _returnvalue (delegate `OnAudioFinished_Event_0`)))))

(event `OnAudioFinished_Event_0`
  (bind _playercontroller (`self.PlayerController`))
  ;[1 1 1] Monolog Samael
  (`/Engine/EditorBlueprintResources/StandardMacros.IsValid` _playercontroller
    (:`Is Valid`
      (`self.EnableInput` _playercontroller null)
      (`self.DelayMotSound`))))

(event `self.OnMotNoise`
  (`GameplayStatics.PlaySoundAtLocation` "/Game/Audio/Ableton_Renders_SFX_and_Synthesen/Swoosh_2_Cue.Swoosh_2_Cue" (620.0 1180.0 80.0) (struct) 1.0 1.0 0.0 null null null null))

(event `self.OnStartFirstDialogueMotAndSamael`
  (bind _playercontroller (`self.PlayerController`))
  ;[1 1 1] Erster Dialog
  (`parent.OnStartFirstDialogueMotAndSamael`)
  (`/Engine/EditorBlueprintResources/StandardMacros.IsValid` _playercontroller
    (:`Is Valid`
      (`CharacterController.StopMoveForDialog` _playercontroller)
      (`self.DisableInput` _playercontroller null)
      (bind _returnvalue (`AddComponent|NODE_AddAudioComponent-7`))
      (`/Engine/EditorBlueprintResources/StandardMacros.IsValid` _returnvalue
        (:`Is Valid`
          (add `AudioComponent.OnAudioFinished` _returnvalue (delegate `OnAudioFinished_Event_1`)))))))

(event `OnAudioFinished_Event_1`
  ;[1 1 1] Erster Dialog
  (bind _returnvalue (`AddComponent|NODE_AddAudioComponent-8`))
  (`/Engine/EditorBlueprintResources/StandardMacros.IsValid` _returnvalue
    (:`Is Valid`
      (add `AudioComponent.OnAudioFinished` _returnvalue (delegate `OnAudioFinished_Event_2`)))))

(event `OnAudioFinished_Event_2`
  ;[1 1 1] Erster Dialog
  (bind _returnvalue (`AddComponent|NODE_AddAudioComponent-9`))
  (`/Engine/EditorBlueprintResources/StandardMacros.IsValid` _returnvalue
    (:`Is Valid`
      (add `AudioComponent.OnAudioFinished` _returnvalue (delegate `OnAudioFinished_Event_3`)))))

(event `OnAudioFinished_Event_3`
  ;[1 1 1] Erster Dialog
  (bind _returnvalue (`AddComponent|NODE_AddAudioComponent-10`))
  (`/Engine/EditorBlueprintResources/StandardMacros.IsValid` _returnvalue
    (:`Is Valid`
      (add `AudioComponent.OnAudioFinished` _returnvalue (delegate `OnAudioFinished_Event_4`)))))

(event `OnAudioFinished_Event_4`
  ;[1 1 1] Erster Dialog
  (bind _returnvalue (`AddComponent|NODE_AddAudioComponent-11`))
  (`/Engine/EditorBlueprintResources/StandardMacros.IsValid` _returnvalue
    (:`Is Valid`
      (add `AudioComponent.OnAudioFinished` _returnvalue (delegate `OnAudioFinished_Event_5`)))))

(event `OnAudioFinished_Event_5`
  (bind _playercontroller (`self.PlayerController`))
  ;[1 1 1] Erster Dialog
  (`/Engine/EditorBlueprintResources/StandardMacros.IsValid` _playercontroller
    (:`Is Valid`
      (`self.EnableInput` _playercontroller null))))

(event `self.OnStartRiddleOne`)

(event `self.OnStartFindTranslation`)

(event `self.OnStartRiddleTwo`)

(event `self.OnStartSecondDialogueMotAndSamael`
  (bind _playercontroller (`self.PlayerController`))
  ;[1 1 1] Zweiter Monolog
  (`parent.OnStartSecondDialogueMotAndSamael`)
  (`/Engine/EditorBlueprintResources/StandardMacros.IsValid` _playercontroller
    (:`Is Valid`
      (`CharacterController.StopMoveForDialog` _playercontroller)
      (`self.DisableInput` _playercontroller _playercontroller)
      (bind _returnvalue (`AddComponent|NODE_AddAudioComponent-18`))
      (`/Engine/EditorBlueprintResources/StandardMacros.IsValid` _returnvalue
        (:`Is Valid`
          (add `AudioComponent.OnAudioFinished` _returnvalue (delegate `OnAudioFinished_Event_6`)))))))

(event `OnAudioFinished_Event_6`
  ;[1 1 1] Zweiter Monolog
  (bind _returnvalue (`AddComponent|NODE_AddAudioComponent-19`))
  (`/Engine/EditorBlueprintResources/StandardMacros.IsValid` _returnvalue
    (:`Is Valid`
      (add `AudioComponent.OnAudioFinished` _returnvalue (delegate `OnAudioFinished_Event_7`)))))

(event `OnAudioFinished_Event_7`
  ;[1 1 1] Zweiter Monolog
  (bind _returnvalue (`AddComponent|NODE_AddAudioComponent-20`))
  (`/Engine/EditorBlueprintResources/StandardMacros.IsValid` _returnvalue
    (:`Is Valid`
      (add `AudioComponent.OnAudioFinished` _returnvalue (delegate `OnAudioFinished_Event_8`)))))

(event `OnAudioFinished_Event_9`
  (bind _playercontroller (`self.PlayerController`))
  ;[1 1 1] Zweiter Monolog
  (`/Engine/EditorBlueprintResources/StandardMacros.IsValid` _playercontroller
    (:`Is Valid`
      (`self.EnableInput` _playercontroller _playercontroller)
      (`self.PlayDoorSound`))))

(event `OnAudioFinished_Event_8`
  ;[1 1 1] Zweiter Monolog
  (bind _returnvalue (`AddComponent|NODE_AddAudioComponent-21`))
  (`/Engine/EditorBlueprintResources/StandardMacros.IsValid` _returnvalue
    (:`Is Valid`
      (add `AudioComponent.OnAudioFinished` _returnvalue (delegate `OnAudioFinished_Event_9`)))))

(event `self.OnStartRiddleThreeAndFour`)

(event `self.OnOpenTrapdoor`
  (`AddComponent|NODE_AddAudioComponent-23`))

(event `self.OnCollectLetter`
  (bind _playercontroller (`self.PlayerController`))
  (`/Engine/EditorBlueprintResources/StandardMacros.IsValid` _playercontroller
    (:`Is Valid`
      (`self.DisableInput` _playercontroller null)
      (bind _returnvalue (`AddComponent|NODE_AddAudioComponent-24`))
      (`/Engine/EditorBlueprintResources/StandardMacros.IsValid` _returnvalue
        (:`Is Valid`
          (add `AudioComponent.OnAudioFinished` _returnvalue (delegate `OnAudioFinished_Event_12`)))))))

(event `OnAudioFinished_Event_12`
  (`self.PlayReadLetterSound`))

(event `self.OnReadLetter`
  (`CharacterController.StopMoveForDialog` (`self.PlayerController`))
  (bind _returnvalue (`AddComponent|NODE_AddAudioComponent-12`))
  (`/Engine/EditorBlueprintResources/StandardMacros.IsValid` _returnvalue
    (:`Is Valid`
      (add `AudioComponent.OnAudioFinished` _returnvalue (delegate `OnAudioFinished_Event_13`))
      (`/Game/Blueprints/Character/BP_Controller_TSS.OpenLetterWidget` (`self.PlayerController`)))))

(event `OnAudioFinished_Event_13`
  (`self.StartLastDialogue`)
  (`/Game/Blueprints/Character/BP_Controller_TSS.CloseLetterWidget` (`self.PlayerController`)))

(event `self.OnLastDialogueMotAndSamael`
  ;[1 1 1] Letzter Monolog
  (`parent.OnLastDialogueMotAndSamael`)
  (bind _returnvalue (`AddComponent|NODE_AddAudioComponent-14`))
  (`/Engine/EditorBlueprintResources/StandardMacros.IsValid` _returnvalue
    (:`Is Valid`
      (add `AudioComponent.OnAudioFinished` _returnvalue (delegate `OnAudioFinished_Event_10`)))))

(event `OnAudioFinished_Event_10`
  ;[1 1 1] Letzter Monolog
  (bind _returnvalue (`AddComponent|NODE_AddAudioComponent-15`))
  (`/Engine/EditorBlueprintResources/StandardMacros.IsValid` _returnvalue
    (:`Is Valid`
      (add `AudioComponent.OnAudioFinished` _returnvalue (delegate `OnAudioFinished_Event_11`)))))

(event `OnAudioFinished_Event_11`
  ;[1 1 1] Letzter Monolog
  (`self.StartMotMonologue`))

(event `self.OnMonologueMot`
  (bind _returnvalue (`AddComponent|NODE_AddAudioComponent-16`))
  (`/Engine/EditorBlueprintResources/StandardMacros.IsValid` _returnvalue
    (:`Is Valid`
      (add `AudioComponent.OnAudioFinished` _returnvalue (delegate `OnAudioFinished_Event_14`))
      (`/Game/Blueprints/Character/BP_Controller_TSS.StartMonologue` (`self.PlayerController`)))))

(event `OnAudioFinished_Event_14`
  (`self.StartSamaelMonologue`)
  (`/Game/Blueprints/Character/BP_Controller_TSS.EndMonologue` (`self.PlayerController`)))

(event `self.OnMonologueSamael`
  (bind _returnvalue (`AddComponent|NODE_AddAudioComponent-17`))
  (add `AudioComponent.OnAudioFinished` _returnvalue (delegate `OnAudioFinished_Event_15`)))

(event `OnAudioFinished_Event_15`
  (bind _playercontroller (`self.PlayerController`))
  (`/Engine/EditorBlueprintResources/StandardMacros.IsValid` _playercontroller
    (:`Is Valid`
      (`self.EnableInput` _playercontroller null))))

(event `self.PlayRiddleSolvedSound`
  (if (`|EnumEquality` (`self.GetCurrentPlayState`) "RiddleFour")
    (`/Game/Blueprints/Character/BP_Controller_TSS.AddItem` (`self.PlayerController`) "/Game/Art/Inventar/Icons/Match.Match"))
  (if true
    (switch `int` (`KismetMathLibrary.RandomInteger` 6)
      (:`0`
        (`AddComponent|NODE_AddAudioComponent-32`))
      (:`1`
        (`AddComponent|NODE_AddAudioComponent-31`))
      (:`2`
        (`AddComponent|NODE_AddAudioComponent-29`))
      (:`3`
        (`AddComponent|NODE_AddAudioComponent-30`))
      (:`4`
        (`AddComponent|NODE_AddAudioComponent-33`))
      (:`5`
        (`AddComponent|NODE_AddAudioComponent-35`)))))

(fn `UserConstructionScript`)