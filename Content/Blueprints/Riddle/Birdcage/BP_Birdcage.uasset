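; Birdcage riddle actor that shows a WBP_BirdCage UI and, once solved, opens the cage door.
; StartRiddle creates or reveals the widget, while StopRiddle and the inventory events toggle its visibility, showing it after a short delay.
; The solved handler broadcasts completion, activates a letter and flags Tick to step the door's yaw down to a limit.
; BeginPlay's widget is never stored, and the solved-event binding sits in unexecuted nodes.
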(event `self.ReceiveBeginPlay`
  (`|CreateWidget` "/Game/Blueprints/Riddle/Widgets/WBP_BirdCage.WBP_BirdCage_C" (`GameplayStatics.GetPlayerController` 0)))

(event `OnCageSolved_Event`
  (`self.BroadCastRiddleFinished`)
  (set `self.RotateDoor` true)
  (`self.ActivateLetter`))

(event `self.ShowInvertory`
  (`KismetSystemLibrary.Delay` 1.3)
  (set `Widget.Visibility` "Visible" (`self.RiddleWidget`)))

(event `self.HideInventory`
  (set `Widget.Visibility` "Collapsed" (`self.RiddleWidget`)))

(event `self.ReceiveTick`
  (params (DeltaSeconds :type "Float (single-precision)"))
  (bind (_returnvalue_roll _returnvalue_pitch _returnvalue_yaw) (`KismetMathLibrary.BreakRotator` (`SceneComponent.K2_GetComponentRotation` (`self.BirdcageDoor`))))
  (if (`self.RotateDoor`)
    (if (>= _returnvalue_yaw -120.0)
      (bind _result (`/Engine/EditorBlueprintResources/StandardMacros.DecrementFloat` _returnvalue_yaw)
        (:`  `
          (`SceneComponent.K2_SetWorldRotation` (`self.BirdcageDoor`) (`KismetMathLibrary.MakeRotator` _returnvalue_roll _returnvalue_pitch _result) false false))))))

(event `self.StartRiddle`
  (bind _riddlewidget (`self.RiddleWidget`))
  (`/Engine/EditorBlueprintResources/StandardMacros.IsValid` _riddlewidget
    (:`Is Valid`
      (set `Widget.Visibility` "Visible" _riddlewidget))
    (:`Is Not Valid`
      (bind _returnvalue (`|CreateWidget` "/Game/Blueprints/Riddle/Widgets/WBP_BirdCage.WBP_BirdCage_C" (`GameplayStatics.GetPlayerController` 0)))
      (bind _output_get (set `self.RiddleWidget` _returnvalue))
      (`UserWidget.AddToViewport` _output_get 0))))

(event `self.StopRiddle`
  (set `Widget.Visibility` "Collapsed" (`self.RiddleWidget`)))

(fn `UserConstructionScript`)