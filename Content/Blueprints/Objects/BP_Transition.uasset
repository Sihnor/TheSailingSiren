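; BP_Transition is a door-like transition object that supplies a transition point and can mark the game's end.
; On BeginPlay it calls UnlockDoor unless IsLocked is set.
; GetTransitionPoint returns TransitionPoint, but for an end door it first tells the BP_Controller_TSS player controller to play the credits.
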(event `self.ReceiveBeginPlay`
  (if (not (`self.IsLocked`))
    (`self.UnlockDoor`)))

(fn `GetTransitionPoint`
  (returns (ReturnValue :type "SceneComponent Object Reference"))
  (if (not (not (`self.IsEndDoor`)))
    (bind _asbp_controller_tss (cast `/Game/Blueprints/Character/BP_Controller_TSS` (`GameplayStatics.GetPlayerController` 0)))
    (`/Game/Blueprints/Character/BP_Controller_TSS.PlayCredits` _asbp_controller_tss))
  (return (`self.TransitionPoint`)))

(fn `UserConstructionScript`)