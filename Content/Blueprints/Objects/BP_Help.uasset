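; BP_Help is an object with a point light that blinks as a hint while the game is in a particular play state.
; The light starts dark at BeginPlay.
; Tick accumulates time and, at each set interval, compares the BP_GameModeTSS current play state to its own state variable, toggling the light intensity between off and on when they match.
; The light is not reset when the state changes.
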(event `self.ReceiveBeginPlay`
  (`LightComponent.SetIntensity` (`self.PointLight`) 0.0))

(event `self.ReceiveTick`
  (params (DeltaSeconds :type "Float (single-precision)"))
  (bind _output_get (set `self.Currentime` (+ DeltaSeconds (`self.Currentime`))))
  (if (>= _output_get (`self.TimeToTick`))
    (set `self.Currentime` 0.0)
    (bind _asbp_game_mode_tss (cast `/Game/Blueprints/GameMode/BP_GameModeTSS` (`GameplayStatics.GetGameMode`)))
    (if (`|EnumEquality` (`self.CurrentGameState`) (`TheSailingSirenGameMode.CurrentPlayState` _asbp_game_mode_tss))
      (`LightComponent.SetIntensity` (`self.PointLight`) (`KismetMathLibrary.SelectFloat` 0.0 10.0 (>= (`LightComponentBase.Intensity` (`self.PointLight`)) 1.0))))))

(fn `UserConstructionScript`)