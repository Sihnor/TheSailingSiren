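; BP_Raven is a raven NPC Blueprint that plays recurring crow caw ambience.
; BeginPlay waits a minute before the first caw, then Tick repeats the sound after random delays of roughly ten to twenty seconds.
; The SetDelay boolean gates Tick so only one delay is pending at a time.
; The cue plays as a non-spatial 2D sound, so the actor's position does not affect it.
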(event `self.ReceiveBeginPlay`
  (set `self.SetDelay` true)
  (`KismetSystemLibrary.Delay` 60.0)
  (`GameplayStatics.PlaySound2D` "/Game/Audio/Ableton_Renders_SFX_and_Synthesen/GameSoundsAssets_GAD_Crow_Indoors_Caw_Groan_Multiple_Cue.GameSoundsAssets_GAD_Crow_Indoors_Caw_Groan_Multiple_Cue" 1.0 1.0 0.0 null null)
  (set `self.SetDelay` false))

(event `self.ReceiveTick`
  (params (DeltaSeconds :type "Float (single-precision)"))
  (if (not (`self.SetDelay`))
    (set `self.SetDelay` true)
    (`KismetSystemLibrary.Delay` (`KismetMathLibrary.Conv_Int64ToDouble` (`KismetMathLibrary.RandomInteger64InRange` 10 21)))
    (`GameplayStatics.PlaySound2D` "/Game/Audio/Ableton_Renders_SFX_and_Synthesen/GameSoundsAssets_GAD_Crow_Indoors_Caw_Groan_Multiple_Cue.GameSoundsAssets_GAD_Crow_Indoors_Caw_Groan_Multiple_Cue" 1.0 1.0 0.0 null null)
    (set `self.SetDelay` false)))

(fn `UserConstructionScript`)