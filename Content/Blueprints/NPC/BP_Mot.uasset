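; BP_Mot is an NPC actor that keeps facing the player and hops between positions supplied by JumpPosition.
; On BeginPlay it locks its own location there, requests a position and listens for changes, each of which starts a jump toward the new XY at zero height.
; Tick animates each jump as two sinusoidally eased segments through a raised intermediate point, using fixed per-frame increments, so speed depends on frame rate.
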(event `self.ReceiveBeginPlay`
  (bind _jumpposition (`self.JumpPosition`))
  (add `JumpPosition.OnPositionChanged` (`self.JumpPosition`) (delegate `OnPositionChanged_Event`))
  (`JumpPosition.LockPosition` _jumpposition (`self.K2_GetActorLocation`))
  (`JumpPosition.SetPosition` _jumpposition))

(event `OnPositionChanged_Event`
  (bind (_returnvalue_x _returnvalue_y) (`KismetMathLibrary.BreakVector` (`JumpPosition.GetPosition` (`self.JumpPosition`))))
  (bind _output_get (set `self.StartJumpPosition` (`self.K2_GetActorLocation`)))
  (set `self.StartJump` true)
  (bind _output_get_2 (set `self.EndJumpPosition` (`KismetMathLibrary.MakeVector` _returnvalue_x _returnvalue_y))))

(event `self.ReceiveTick`
  (params (DeltaSeconds :type "Float (single-precision)"))
  (bind _startjumpposition (`self.StartJumpPosition`))
  (`parent.ReceiveTick` DeltaSeconds)
  (`self.K2_SetActorRotation` (`KismetMathLibrary.FindLookAtRotation` (`self.K2_GetActorLocation`) (`PlayerPosition.GetPlayerPosition` (`self.PlayerPosition`))))
  (if (`self.StartJump`)
    (if (not (`self.FirstHalf`))
      (bind _output_get (set `self.MiddleJumpPosition` (+ (+ (/ (- (`self.EndJumpPosition`) _startjumpposition) 1.5) _startjumpposition) (0.0 0.0 200.0))))
      (`self.K2_SetActorLocation` (`|EaseFunction` "SinusoidalInOut" (`self.index`) (`self.StartJumpPosition`) _output_get))
      (bind _output_get_2 (set `self.Index` (+ (`self.Index`) 0.03)))
      (if (>= _output_get_2 1.0)
        (set `self.FirstHalf` true)
        (set `self.Index` 0.0))
      (else
        (`self.K2_SetActorLocation` (`|EaseFunction` "SinusoidalInOut" (`self.index`) (`self.MiddleJumpPosition`) (`self.EndJumpPosition`)))
        (bind _output_get_3 (set `self.Index` (+ (`self.Index`) 0.05)))
        (if (>= _output_get_3 1.0)
          (set `self.StartJump` false)
          (set `self.index` 0.0)
          (set `self.FirstHalf` false))))))

(fn `UserConstructionScript`)